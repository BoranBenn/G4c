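; Actor Blueprint that makes objects fall at random by switching on their gravity over time.
; From BeginPlay, a looping timer calls Düsme every four seconds to enable gravity on a random pick from four array entries, which can repeat.
; A second looping timer decrements the Timer counter each second.
; Düsme clears both timers only if Timer is exactly zero when it runs.
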(event `self.ReceiveBeginPlay`
  (bind _returnvalue (`KismetSystemLibrary.K2_SetTimerDelegate` (delegate `Düsme`) 4.0 true))
  (set `self.NewVar` _returnvalue)
  (bind _returnvalue_2 (`KismetSystemLibrary.K2_SetTimerDelegate` (delegate `CustomEvent`) 1.0 true)))

(event `CustomEvent`
  (`/Engine/EditorBlueprintResources/StandardMacros.DecrementInt` (`self.timer`)))

(event `Düsme`
  (`PrimitiveComponent.SetEnableGravity` (`|GetArrayItem` (`|MakeArray` null :!type "PrimitiveComponent Object Reference") (`KismetMathLibrary.RandomInteger` 4)) true)
  (if (== (`self.timer`) 0)
    (`KismetSystemLibrary.K2_ClearAndInvalidateTimerHandle` (`self.NewVar`))
    (`KismetSystemLibrary.K2_ClearAndInvalidateTimerHandle` (stale `self.ReceiveBeginPlay` _returnvalue_2))))

(fn `UserConstructionScript`)