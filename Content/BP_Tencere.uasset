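; BP_Tencere is a player-controlled object that slides its Cube sideways along the world Y axis with the A and D keys.
; On BeginPlay it switches the player's view to the target held in NewVar.
; A key press sets a direction and starts a fast looping timer on MoveLeft, which offsets the Cube in both directions without sweep.
; Releasing either key re-sets that shared timer with zero time, stopping movement.
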(event `self.ReceiveBeginPlay`
  (`PlayerController.SetViewTargetWithBlend` (`GameplayStatics.GetPlayerController` 0) (`self.NewVar`) 0.0 "VTBlend_Linear" 0.0 false))

(event `Key|D`
  (params (Key :type "Key Structure"))
  (:`Pressed`
    (set `self.Timer` 0.01)
    (set `self.Direction` (0.0 2.0 0.0) :!label _label)
    (`KismetSystemLibrary.K2_SetTimerDelegate` (delegate `MoveLeft`) (`self.Timer`) true))
  (:`Released`
    (set `self.Timer` 0.0)
    (goto _label)))

(event `Key|A`
  (params (Key :type "Key Structure"))
  (:`Pressed`
    (set `self.Timer` 0.01)
    (set `self.Direction` (0.0 -2.0 0.0) :!label _label_2)
    (`KismetSystemLibrary.K2_SetTimerDelegate` (delegate `MoveLeft`) (`self.Timer`) true))
  (:`Released`
    (set `self.Timer` 0.0)
    (goto _label_2)))

(event `MoveLeft`
  (bind _cube (`self.Cube`))
  (bind _returnvalue_location (`KismetMathLibrary.BreakTransform` (`SceneComponent.K2_GetComponentToWorld` _cube)))
  (`SceneComponent.K2_SetWorldLocation` _cube (+ _returnvalue_location (`self.Direction`)) false false))

(fn `UserConstructionScript`)