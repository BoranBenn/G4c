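; BP_Düsecekler is a timed spawner that drops BP_Food actors into the level from above.
; A looping timer spawns food at one of two mirrored positions, passing a random FoodArray entry as Owner.
; A second looping timer decrements the Timer countdown each second.
; NewFunction enables gravity on each food's cube and clears both timers only if Timer equals exactly zero at that spawn.
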(event `self.ReceiveBeginPlay`
  (bind _returnvalue (`KismetSystemLibrary.K2_SetTimerDelegate` (delegate `Düsme`) 3.0 true))
  (set `self.NewVar` _returnvalue)
  (bind _returnvalue_2 (`KismetSystemLibrary.K2_SetTimerDelegate` (delegate `CustomEvent`) 1.0 true))
  (set `self.NewVar_1` _returnvalue_2))

(event `CustomEvent`
  (`/Engine/EditorBlueprintResources/StandardMacros.DecrementInt` (`self.timer`)))

(event `Düsme`
  (if (`KismetMathLibrary.RandomBool`)
    (bind _returnvalue (`|SpawnActorFromClass` "/Game/Blueprints/Food/BP_Food.BP_Food_C" (`KismetMathLibrary.MakeTransform` (160.0 350.0 600.0)) "Undefined" "MultiplyWithRoot" (`|GetArrayItem` (`/Game/Blueprints/Food/BP_FoodSetter.FoodArray` (`self.NewVar_0`)) (`KismetMathLibrary.RandomInteger` 2)) null))
    (`self.NewFunction` _returnvalue)
    (else
      (bind _returnvalue_2 (`|SpawnActorFromClass` "/Game/Blueprints/Food/BP_Food.BP_Food_C" (`KismetMathLibrary.MakeTransform` (160.0 -350.0 600.0)) "Undefined" "MultiplyWithRoot" (`|GetArrayItem` (`/Game/Blueprints/Food/BP_FoodSetter.FoodArray` (`self.NewVar_0`)) (`KismetMathLibrary.RandomInteger` 2)) null))
      (`self.NewFunction` _returnvalue_2))))

(fn `NewFunction`
  (params (self2 :type "/Game/Blueprints/Food/BP_Food Object Reference"))
  (`PrimitiveComponent.SetEnableGravity` (`/Game/Blueprints/Food/BP_Food.Cube` self2) true)
  (if (== (`self.timer`) 0)
    (`KismetSystemLibrary.K2_ClearAndInvalidateTimerHandle` (`self.NewVar`))
    (`KismetSystemLibrary.K2_ClearAndInvalidateTimerHandle` (`self.NewVar_1`))))

(fn `UserConstructionScript`)