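; Sound manager actor that plays 2D ambience for a kitchen first level and a street second level, plus a collision sound.
; BeginPlay loops a FlipFlop that alternately spawns the two kitchen cues, stacking several at once.
; Level2Ses calls Stop on AktifSes, whose assignments are unconnected, then spawns one street cue through another FlipFlop.
; Carpisma spawns the collision sound with a heavily boosted volume multiplier.
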(event `self.ReceiveBeginPlay`
  (`self.NewFunction`))

(event `Level2Ses`
  (`self.NewFunction_0`))

(event `Carpisma`
  (bind _returnvalue (`GameplayStatics.SpawnSound2D` "/Game/audio/potlarssss.potlarssss" 1.0 1.0 0.0 null))
  (`AudioComponent.SetVolumeMultiplier` _returnvalue 50.0))

(fn `NewFunction`
  (set `self.lev1` true)
  (if (== (`self.lev1`) true)
    (for _ (range 4) :!label _label
      (`/Engine/EditorBlueprintResources/StandardMacros.FlipFlop`
        (:`A`
          (bind _returnvalue (`GameplayStatics.SpawnSound2D` "/Game/audio/Mutfak_Sesi_2_Cue.Mutfak_Sesi_2_Cue" 1.0 1.0 0.0 null)))
        (:`B`
          (bind _returnvalue_2 (`GameplayStatics.SpawnSound2D` "/Game/audio/Mustafk_Sesi_1_Cue.Mustafk_Sesi_1_Cue" 1.0 1.0 0.0 null)))))
    (else
      (goto _label :!via `Break`))))

(fn `NewFunction_0`
  (set `self.lev1` false)
  (`AudioComponent.Stop` (`self.AktifSes`))
  (`/Engine/EditorBlueprintResources/StandardMacros.FlipFlop`
    (:`A`
      (bind _returnvalue (`GameplayStatics.SpawnSound2D` "/Game/audio/Sokak_Sesi_Cue1.Sokak_Sesi_Cue1" 1.0 1.0 0.0 null)))
    (:`B`
      (bind _returnvalue_2 (`GameplayStatics.SpawnSound2D` "/Game/audio/Sokak_Sesi_Cue.Sokak_Sesi_Cue" 1.0 1.0 0.0 null)))))

(fn `UserConstructionScript`)