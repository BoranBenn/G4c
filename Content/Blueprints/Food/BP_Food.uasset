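; BP_Food is a physics-driven food item that randomly appears as a piece of meat, a potato or an eggplant.
; The Construction Script picks one of the three meshes at random and assigns its matching materials.
; On BeginPlay the Cube mesh receives a strong one-time impulse along its right vector, with the direction chosen by the sign of world Y so opposite sides launch in opposite directions.
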(event `self.ReceiveBeginPlay`
  (bind _cube (`self.Cube`))
  (bind _returnvalue (`SceneComponent.GetRightVector` (`self.Cube`)))
  (if (>= (.y (.location (`self.GetTransform`))) 0.0)
    (`PrimitiveComponent.AddImpulse` _cube (* _returnvalue -50000) "None" false)
    (else
      (`PrimitiveComponent.AddImpulse` _cube (* _returnvalue 50000) "None" false))))

(fn `UserConstructionScript`
  (bind _cube (`self.Cube`))
  (bind _cube_2 (`self.Cube`))
  (switch `int` (`KismetMathLibrary.RandomIntegerInRange` 0 2)
    (:`0`
      (`StaticMeshComponent.SetStaticMesh` _cube "/Game/Assets/Food/EtParcasi.EtParcasi")
      (`PrimitiveComponent.SetMaterial` _cube_2 1 "/Game/Assets/Food/beyaz.beyaz")
      (`PrimitiveComponent.SetMaterial` _cube_2 0 "/Game/Assets/Food/kirmizi.kirmizi"))
    (:`1`
      (`StaticMeshComponent.SetStaticMesh` _cube "/Game/Assets/Food/Patates.Patates")
      (`PrimitiveComponent.SetMaterial` (`self.Cube`) 0 "/Game/Assets/Food/kahverengi.kahverengi"))
    (:`2`
      (`StaticMeshComponent.SetStaticMesh` _cube "/Game/Assets/Food/patlican.patlican")
      (`PrimitiveComponent.SetMaterial` (`self.Cube`) 0 "/Game/Assets/Food/mor.mor"))))