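; BP_Cameraa switches the player's view to a referenced camera when the second level signals through an event dispatcher.
; On BeginPlay it binds to the OnLevel2 dispatcher on SecondLevelRef, whose event blends player 0's view target to CameraRef over a short transition.
; The Move event is empty, and the camera-repositioning and timer nodes are unconnected, so they never run.
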(event `self.ReceiveBeginPlay`
  (add `/Game/Blueprints/BP_SecondLevel.OnLevel2` (`self.SecondLevelRef`) (delegate `OnLevel2_Event`)))

(event `OnLevel2_Event`
  (`PlayerController.SetViewTargetWithBlend` (`GameplayStatics.GetPlayerController` 0) (`self.CameraRef`) 2.0 "VTBlend_Linear" 0.0 false))

(event `Move`)

(fn `UserConstructionScript`)