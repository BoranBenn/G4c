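; BP_El is a level 2 player pawn that slides a cube sideways and destroys any BP_Food overlapping its box.
; When SecondRef signals level 2, it waits briefly, possesses itself and switches to CameraRef.
; A and D drive a looping timer on MoveLeft, which handles both directions; a zero time stops it, and releasing one key resumes the other if held.
; MoveLeft nudges the cube back when it leaves the Y limits.
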(event `self.ReceiveBeginPlay`
  (add `/Game/Blueprints/BP_SecondLevel.OnLevel2` (`self.SecondRef`) (delegate `OnLevel2_Event`)))

(event `OnLevel2_Event`
  (`KismetSystemLibrary.Delay` 2.0)
  (`Controller.Possess` (`GameplayStatics.GetPlayerController` 0) self)
  (`PlayerController.SetViewTargetWithBlend` (`GameplayStatics.GetPlayerController` 0) (`self.CameraRef`) 0.0 "VTBlend_Linear" 0.0 false))

(event `Key|D`
  (params (Key :type "Key Structure"))
  (:`Pressed`
    (set `self.DPressed` true)
    (set `self.RightTimer` 0.01 :!label _label)
    (set `self.Direction` (0.0 5.0 0.0))
    (`KismetSystemLibrary.K2_SetTimerDelegate` (delegate `MoveLeft`) (`self.RightTimer`) true :!label _label_2))
  (:`Released`
    (set `self.DPressed` false)
    (set `self.RightTimer` 0.0)
    (if (`self.APressed`)
      (set `self.LeftTimer` 0.01 :!label _label_3)
      (set `self.Direction` (0.0 -5.0 0.0))
      (`KismetSystemLibrary.K2_SetTimerDelegate` (delegate `MoveLeft`) (`self.LeftTimer`) true :!label _label_4)
      (else
        (goto _label_2)))))

(event `Key|A`
  (params (Key :type "Key Structure"))
  (:`Pressed`
    (set `self.APressed` true)
    (goto _label_3))
  (:`Released`
    (set `self.APressed` false)
    (set `self.LeftTimer` 0.0)
    (if (`self.DPressed`)
      (goto _label)
      (else
        (goto _label_4)))))

(event `MoveLeft`
  (bind _cube (`self.Cube`))
  (bind _cube_2 (`self.Cube`))
  (bind (_returnvalue_x _returnvalue_y _returnvalue_z) (`KismetMathLibrary.BreakVector` (`SceneComponent.K2_GetComponentLocation` (`self.Cube`))))
  (bind (_returnvalue_x_2 _returnvalue_y_2) (`KismetMathLibrary.BreakVector` (`SceneComponent.K2_GetComponentLocation` (`self.Cube`))))
  (bind _returnvalue_location (`KismetMathLibrary.BreakTransform` (`SceneComponent.K2_GetComponentToWorld` _cube_2)))
  (if (and (<= _returnvalue_y_2 430.0) (>= _returnvalue_y_2 -550.0))
    (`SceneComponent.K2_SetWorldLocation` _cube_2 (+ _returnvalue_location (`self.Direction`)) false false)
    (elif (> _returnvalue_y 0.0)
      (`SceneComponent.K2_SetWorldLocation` _cube (`KismetMathLibrary.MakeVector` _returnvalue_x (+ _returnvalue_y -1.0) _returnvalue_z) false false)
      (else
        (`SceneComponent.K2_SetWorldLocation` _cube (`KismetMathLibrary.MakeVector` _returnvalue_x (+ _returnvalue_y 1.0) _returnvalue_z) false false)))))

(event `self.Box.OnComponentBeginOverlap`
  (params (OverlappedComponent :type "PrimitiveComponent Object Reference") (OtherActor :type "Actor Object Reference") (OtherComp :type "PrimitiveComponent Object Reference") (OtherBodyIndex :type Integer) (bFromSweep :type Boolean) (SweepResult :type "HitResult Structure (by ref)"))
  (if (== (`GameplayStatics.GetObjectClass` OtherActor) "/Game/Blueprints/Food/BP_Food.BP_Food_C")
    (bind _asbp_food (cast `/Game/Blueprints/Food/BP_Food` OtherActor))
    (`self.K2_DestroyActor` _asbp_food)))

(fn `UserConstructionScript`)