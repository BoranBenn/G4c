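; BP_Kacirilanlar is a hidden-mesh catcher that records missed BP_Food items and drops them again in level 2.
; Overlaps on component R add each unique food to the Kacanlar array.
; SecLev's OnLevel2 dispatcher starts a looping timer that enables physics on the oldest stored food's Cube and removes it from the array.
; When a tick finds the array empty, it clears the timer and opens EndScreen.
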(event `self.ReceiveBeginPlay`
  (`SceneComponent.SetVisibility` (`self.mesh`) false false)
  (add `/Game/Blueprints/BP_SecondLevel.OnLevel2` (`self.SecLev`) (delegate `OnLevel2_Event`)))

(event `OnLevel2_Event`
  (bind _returnvalue (`KismetSystemLibrary.K2_SetTimerDelegate` (delegate `ikincidusme`) 3.0 true))
  (set `self.NewVar` _returnvalue))

(event `ikincidusme`
  (bind _kacanlar (`self.Kacanlar`))
  (bind _output (`|GetArrayItem` _kacanlar))
  (if (`KismetArrayLibrary.Array_IsEmpty` _kacanlar)
    (`KismetSystemLibrary.K2_ClearAndInvalidateTimerHandle` (`self.NewVar`))
    (`GameplayStatics.OpenLevelBySoftObjectPtr` "/Game/Levels/EndScreen.EndScreen")
    (else
      (`PrimitiveComponent.SetSimulatePhysics` (`/Game/Blueprints/Food/BP_Food.Cube` _output) true)
      (`KismetArrayLibrary.Array_RemoveItem` _kacanlar _output)
      (`KismetSystemLibrary.PrintString` "Hello"))))

(event `self.r.OnComponentBeginOverlap`
  (params (OverlappedComponent :type "PrimitiveComponent Object Reference") (OtherActor :type "Actor Object Reference") (OtherComp :type "PrimitiveComponent Object Reference") (OtherBodyIndex :type Integer) (bFromSweep :type Boolean) (SweepResult :type "HitResult Structure (by ref)"))
  (bind _kacanlar (`self.Kacanlar`))
  (if (== (`GameplayStatics.GetObjectClass` OtherActor) "/Game/Blueprints/Food/BP_Food.BP_Food_C")
    (bind _asbp_food (cast `/Game/Blueprints/Food/BP_Food` OtherActor))
    (if (not (`KismetArrayLibrary.Array_Contains` _kacanlar _asbp_food))
      (`KismetArrayLibrary.Array_Add` _kacanlar _asbp_food)
      (`KismetSystemLibrary.PrintString` (`KismetSystemLibrary.GetDisplayName` _asbp_food)))))

(fn `UserConstructionScript`)