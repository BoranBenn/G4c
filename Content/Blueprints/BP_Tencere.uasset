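; BP_Tencere is a player-steered catcher that slides sideways along Y and destroys the referenced Top actor when it overlaps its Box.
; BeginPlay switches the player's view to a referenced target.
; A and D set the direction of one looping timer event that steps the Cube without sweeping.
; Releasing a key hands movement to the other if still held, otherwise a zero interval clears the timer.
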(event `self.ReceiveBeginPlay`
  (`PlayerController.SetViewTargetWithBlend` (`GameplayStatics.GetPlayerController` 0) (`self.NewVar`) 0.0 "VTBlend_Linear" 0.0 false))

(event `Key|SpaceBar`
  (params (Key :type "Key Structure")))

(event `Key|D`
  (params (Key :type "Key Structure"))
  (:`Pressed`
    (set `self.DPressed` true)
    (set `self.RightTimer` 0.01 :!label _label)
    (set `self.Direction` (0.0 2.0 0.0))
    (`KismetSystemLibrary.K2_SetTimerDelegate` (delegate `MoveLeft`) (`self.RightTimer`) true :!label _label_2))
  (:`Released`
    (set `self.DPressed` false)
    (set `self.RightTimer` 0.0)
    (if (`self.APressed`)
      (set `self.LeftTimer` 0.01 :!label _label_3)
      (set `self.Direction` (0.0 -2.0 0.0))
      (`KismetSystemLibrary.K2_SetTimerDelegate` (delegate `MoveLeft`) (`self.LeftTimer`) true :!label _label_4)
      (else
        (goto _label_2)))))

(event `Key|A`
  (params (Key :type "Key Structure"))
  (:`Pressed`
    (set `self.APressed` true)
    (goto _label_3))
  (:`Released`
    (set `self.APressed` false)
    (set `self.LeftTimer` 0.0)
    (if (`self.DPressed`)
      (goto _label)
      (else
        (goto _label_4)))))

(event `MoveLeft`
  (bind _cube (`self.Cube`))
  (bind _returnvalue_location (`KismetMathLibrary.BreakTransform` (`SceneComponent.K2_GetComponentToWorld` _cube)))
  (`SceneComponent.K2_SetWorldLocation` _cube (+ _returnvalue_location (`self.Direction`)) false false))

(event `self.Box.OnComponentBeginOverlap`
  (params (OverlappedComponent :type "PrimitiveComponent Object Reference") (OtherActor :type "Actor Object Reference") (OtherComp :type "PrimitiveComponent Object Reference") (OtherBodyIndex :type Integer) (bFromSweep :type Boolean) (SweepResult :type "HitResult Structure (by ref)"))
  (bind _top (`self.Top`))
  (if (== OtherActor _top)
    (`self.K2_DestroyActor` _top)))

(fn `UserConstructionScript`)