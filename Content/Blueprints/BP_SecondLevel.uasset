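; BP_SecondLevel handles the transition to the second level through its GravityFalls event.
; The event finds the BP_Kacirilanlar actor and stops physics simulation on the cube of each entry in its Kacanlar array.
; Both the loop body and its completion then disable collision on a referenced mesh, fire the OnLevel2 dispatcher and call Level2Ses on another reference, so these steps repeat per element.
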(event `GravityFalls`
  (bind _outactors (`GameplayStatics.GetAllActorsOfClass` "/Game/Blueprints/BP_Kacirilanlar.BP_Kacirilanlar_C"))
  (bind _asbp_kacirilanlar (cast `/Game/Blueprints/BP_Kacirilanlar` (`|GetArrayItem` _outactors)))
  (for _array_element (`/Game/Blueprints/BP_Kacirilanlar.Kacanlar` _asbp_kacirilanlar)
    (`PrimitiveComponent.SetSimulatePhysics` (`/Game/Blueprints/Food/BP_Food.Cube` _array_element) false)
    (`PrimitiveComponent.SetCollisionEnabled` (`/Game/Blueprints/BP_Kacirilanlar.mesh` (`self.NewVar`)) "NoCollision" :!label _label)
    (`self.OnLevel2`)
    (`/Game/Blueprints/BP_Sound.Level2Ses` (`self.NewVar_0`)))
  (goto _label))

(event `self.ReceiveBeginPlay`)

(fn `UserConstructionScript`)